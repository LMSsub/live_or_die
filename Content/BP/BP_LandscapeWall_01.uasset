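; Landscape wall actor that builds a wall from spline mesh components along an editable spline in its construction script.
; With ActivateLineTrace on, vertical Visibility traces first snap each spline point to the surface hit.
; Each segment fits a whole number of WallMesh copies based on its X bounds, stretched evenly to fill it, with tangents clamped to piece length.
; Segments shorter than one mesh width get no wall.
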(fn `Get_Current_mesh_count`
  (returns (ReturnValue :type Boolean))
  (bind _output_get (set `self.Current_mesh_count` (`KismetMathLibrary.FFloor` (`KismetMathLibrary.SafeDivide` (`self.Current_spline_length`) (`self.Wall_Width`)))))
  (return (> _output_get 0)))

(fn `Get_Current_spline_Length`
  (bind _returnvalue (`SplineComponent.GetDistanceAlongSplineAtSplinePoint` (`self.Spline`) (`self.Current_Point_index`)))
  (set `self.Cuurrent_Ponit_distance` _returnvalue)
  (set `self.Current_spline_length` (- (`SplineComponent.GetDistanceAlongSplineAtSplinePoint` (`self.Spline`) (+ (`self.Current_Point_index`) 1)) _returnvalue)))

(fn `Get_wall_width`
  (bind (_returnvalue_min _returnvalue_max) (break `Box` (`StaticMesh.GetBoundingBox` (`self.Wall_Mesh`))))
  (bind _returnvalue_x (`KismetMathLibrary.BreakVector` (- _returnvalue_max _returnvalue_min)))
  (set `self.Wall_Width` _returnvalue_x))

(fn `UserConstructionScript`
  (`|ExecutionSequence`
    (:`then_0`
      (if (`self.Activate_Line_Trace`)
        (for _index (range (`SplineComponent.GetNumberOfSplinePoints` (`self.Spline`)))
          (bind (_returnvalue_x _returnvalue_y _returnvalue_z) (`KismetMathLibrary.BreakVector` (`SplineComponent.GetLocationAtSplinePoint` (`self.Spline`) _index "World")))
          (bind (_outhit _returnvalue) (`KismetSystemLibrary.LineTraceSingle` :`Start` (`KismetMathLibrary.MakeVector` _returnvalue_x _returnvalue_y (+ _returnvalue_z 10000.0)) :`End` (`KismetMathLibrary.MakeVector` _returnvalue_x _returnvalue_y (- _returnvalue_z 10000.0)) :`TraceChannel` "TraceTypeQuery1" :`DrawTime` 20.0))
          (if _returnvalue
            (`SplineComponent.SetLocationAtSplinePoint` (`self.Spline`) _index (`.Location` (`GameplayStatics.BreakHitResult` _outhit)) "World" true)))))
    (:`then_1`
      (`/Engine/EditorBlueprintResources/StandardMacros.IsValid` (`self.Wall_Mesh`)
        (:`Is Valid`
          (`self.Get_wall_width`)
          (for _index_2 (range (+ (- (`SplineComponent.GetNumberOfSplinePoints` (`self.Spline`)) 2) 1))
            (set `self.Current_Point_index` _index_2)
            (`self.Get_Current_spline_Length`)
            (bind _returnvalue_2 (`self.Get_Current_mesh_count`))
            (if _returnvalue_2
              (set `self.Currnet_modified_mesh_width` (/ (`self.Current_spline_length`) (`self.Current_mesh_count`)))
              (for _index_3 (range (`self.Current_mesh_count`))
                (bind _returnvalue_3 (`AddComponent|NODE_AddSplineMeshComponent-0`))
                (bind _returnvalue_4 (+ (* _index_3 (`self.Currnet_modified_mesh_width`)) (`self.Cuurrent_Ponit_distance`)))
                (bind _returnvalue_5 (+ (* (+ _index_3 1) (`self.Currnet_modified_mesh_width`)) (`self.Cuurrent_Ponit_distance`)))
                (`SplineMeshComponent.SetStartAndEnd` _returnvalue_3 (`SplineComponent.GetLocationAtDistanceAlongSpline` (`self.Spline`) _returnvalue_4 "Local") (`KismetMathLibrary.ClampVectorSize` (`SplineComponent.GetTangentAtDistanceAlongSpline` (`self.Spline`) _returnvalue_4 "Local") 1.0 (`self.Currnet_modified_mesh_width`)) (`SplineComponent.GetLocationAtDistanceAlongSpline` (`self.Spline`) _returnvalue_5 "Local") (`KismetMathLibrary.ClampVectorSize` (`SplineComponent.GetTangentAtDistanceAlongSpline` (`self.Spline`) _returnvalue_5 "Local") 1.0 (`self.Currnet_modified_mesh_width`)) true)
                (`StaticMeshComponent.SetStaticMesh` _returnvalue_3 (`self.Wall_Mesh`))
                (`SceneComponent.K2_AttachToComponent` _returnvalue_3 (`self.Spline`) "None" "KeepRelative" "KeepRelative" "KeepRelative" true)))))))))